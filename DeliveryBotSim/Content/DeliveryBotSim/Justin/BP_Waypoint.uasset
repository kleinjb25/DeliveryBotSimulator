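; BP_Waypoint is a waypoint actor that displays the player's distance to it in yards.
; On BeginPlay it casts its widget component's widget to WP_Waypoint and caches that widget's Distance text element.
; Every Tick it measures the distance to player pawn 0, converts centimeters to truncated whole yards, and writes the value with a "yd" suffix into the text.
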(event `self.ReceiveBeginPlay`
  (bind _aswp_waypoint (cast `/Game/DeliveryBotSim/Justin/WP_Waypoint` (`WidgetComponent.GetWidget` (`self.Widget`))))
  (set `self.Distance` (`/Game/DeliveryBotSim/Justin/WP_Waypoint.distance` _aswp_waypoint)))

(event `self.ReceiveTick`
  (params (DeltaSeconds :type "Float (single-precision)"))
  (set `TextBlock.Text` (`KismetTextLibrary.Conv_StringToText` (`KismetStringLibrary.Concat_StrStr` (`KismetStringLibrary.Conv_IntToString` (`KismetMathLibrary.FTrunc` (/ (`KismetMathLibrary.Vector_Distance` (`self.K2_GetActorLocation`) (`self.K2_GetActorLocation` (`GameplayStatics.GetPlayerPawn` 0))) 91.44))) " yd")) (`self.Distance`)))

(fn `UserConstructionScript`)