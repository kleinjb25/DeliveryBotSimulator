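; Parent car actor for the delivery bot sim that acts as looping traffic and a lethal hazard for the player.
; Tick moves it along a local direction with a swept offset, accumulates distance travelled, and teleports it back to its BeginPlay location past the maximum distance.
; Overlapping the third-person character reports a death with a scolding message to the first ThirdPerson_UI widget found and plays a crash sound.
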(event `self.ReceiveBeginPlay`
  (set `self.startlocation` (`self.K2_GetActorLocation` self)))

(event `self.ReceiveActorBeginOverlap`
  (params (OtherActor :type "Actor Object Reference"))
  (bind _asbp_third_person_character (cast `/Game/ThirdPerson/Blueprints/BP_ThirdPersonCharacter` OtherActor))
  (bind _foundwidgets (`WidgetBlueprintLibrary.GetAllWidgetsOfClass` "/Game/DeliveryBotSim/ConnorBrown/ThirdPerson_UI.ThirdPerson_UI_C"))
  (`/Game/DeliveryBotSim/ConnorBrown/ThirdPerson_UI.OrderCompleteOrDied` (`|GetArrayItem` _foundwidgets) _asbp_third_person_character true "Did you forget to look both ways before crossing the street? It's first grade knowledge, player!")
  (`GameplayStatics.PlaySoundAtLocation` "/Game/DeliveryBotSim/Justin/SoundEffects/carCrash.carCrash" (`self.K2_GetActorLocation`) (struct) 1.0 1.0 0.0 null null null null))

(event `self.ReceiveTick`
  (params (DeltaSeconds :type "Float (single-precision)"))
  (bind _returnvalue (* (* DeltaSeconds (`self.speed`)) (`self.direction`)))
  (`self.K2_AddActorLocalOffset` _returnvalue true)
  (bind _output_get (set `self.currdistance` (+ (`KismetMathLibrary.VSize` _returnvalue) (`self.currdistance`))))
  (if (> _output_get (`self.maxdistance`))
    (`self.K2_SetActorLocation` (`self.startlocation`) false true)
    (set `self.currdistance` 0.0)))

(fn `UserConstructionScript`)