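; Female student NPC that can chase down the delivery player and end the run with a death message.
; It issues random roam moves, though Tick halts movement until PawnSensing randomly triggers a chase.
; On reaching the player, it plays a montage, then a sphere trace and CanAttack gate the UI death call.
; Player overlap, gated by a NAND of speed and physics checks, makes it scream, ragdoll and despawn.
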(event `self.ReceiveTick`
  (params (DeltaSeconds :type "Float (single-precision)"))
  (if (not (`self.IsSeeingPlayer`))
    (`MovementComponent.StopMovementImmediately` (`self.CharacterMovement`))))

(event `self.ReceiveBeginPlay`
  (`KismetSystemLibrary.RetriggerableDelay` (`KismetMathLibrary.RandomFloatInRange` 0.0 5.0) :!label _label)
  (`|AIMoveTo` self (`NavigationSystemV1.K2_GetRandomReachablePointInRadius` (`self.K2_GetActorLocation`) 1000.0 null null) null
    (:`then`
      (goto _label))))

(event `self.PawnSensing.OnSeePawn`
  (params (Pawn :type "Pawn Object Reference"))
  (if (<= (`KismetMathLibrary.RandomFloatInRange` 0.0 5.0) 2.0)
    (set `self.IsSeeingPlayer` true)
    (`self.FollowPlayer`)))

(event `FollowPlayer`
  (if (`self.IsSeeingPlayer`)
    (`|AIMoveTo` self (0.0 0.0 0.0) (`GameplayStatics.GetPlayerCharacter` 0) 10.0
      (:`OnSuccess`
        (bind _returnvalue (`self.PlayAnimMontage` null))
        (`KismetSystemLibrary.Delay` _returnvalue)
        (bind (_outhit _returnvalue_2) (`KismetSystemLibrary.SphereTraceSingleForObjects` (`self.K2_GetActorLocation`) (`self.K2_GetActorLocation` (`GameplayStatics.GetPlayerCharacter` 0)) 0.01 (`|MakeArray` "ObjectTypeQuery3" :!type "EObjectTypeQuery Enum")))
        (if (and _returnvalue_2 (`self.canAttack?`))
          (bind _foundwidgets (`WidgetBlueprintLibrary.GetAllWidgetsOfClass` "/Game/DeliveryBotSim/ConnorBrown/ThirdPerson_UI.ThirdPerson_UI_C"))
          (bind _returnvalue_3 (`GameplayStatics.GetActorOfClass` "/Game/ThirdPerson/Blueprints/BP_ThirdPersonCharacter.BP_ThirdPersonCharacter_C"))
          (`/Game/DeliveryBotSim/ConnorBrown/ThirdPerson_UI.OrderCompleteOrDied` (`|GetArrayItem` _foundwidgets) _returnvalue_3 true "Damn, these students must really hate you!"))
        (set `self.canAttack?` false)
        (`KismetSystemLibrary.Delay` 4.0)))
    (else
      (set `self.IsSeeingPlayer` false))))

(event `self.ReceiveActorBeginOverlap`
  (params (OtherActor :type "Actor Object Reference"))
  (bind _asbp_third_person_character (cast `/Game/ThirdPerson/Blueprints/BP_ThirdPersonCharacter` OtherActor))
  (if (`KismetMathLibrary.BooleanNAND` (>= (`KismetMathLibrary.VSizeXY` (`CharacterMovementComponent.GetLastUpdateVelocity` (`Character.CharacterMovement` _asbp_third_person_character))) 500.0) (`SceneComponent.IsSimulatingPhysics` (`self.Mesh`) "None"))
    (`GameplayStatics.PlaySoundAtLocation` "/Game/DeliveryBotSim/Justin/SoundEffects/randomFemaleScream.randomFemaleScream" (`self.K2_GetActorLocation`) (struct) 1.0 1.0 0.0 null null null null)
    (`PrimitiveComponent.SetSimulatePhysics` (`self.Mesh`) true)
    (set `self.canAttack?` false)
    (`KismetSystemLibrary.Delay` 10.0)
    (`self.K2_DestroyActor`)))

(fn `UserConstructionScript`)